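; Tracked vehicle Blueprint that turns player axis input into drive, steering and brake values.
; The forward/backward axis sets opposite left and right wheel coefficients, despite its name.
; The right/left axis feeds auto-handling throttle when AutoGearBox is on, otherwise setting forward coefficient and equal brake ratios.
; Non-zero input clears sleep mode, and a custom event starts or clears a looping gearbox update timer.
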(event `InputAxis|VehicleForwardBackward`
  (params (AxisValue :type "Float (single-precision)"))
  ;[1 1 1] Vehicle Movement Controls
  (bind _output_get (set `self.WheelRightCoefficient` AxisValue))
  (set `self.WheelLeftCoefficient` (* -1 _output_get))
  (if (or (!= AxisValue 0.0) (!= (stale `InputAxis|VehicleRightLeft` AxisValue) 0.0)) :!label _label
    (set `self.SleepMode` false)
    (set `self.SleepDelayTimer` 0.0)))

(event `InputAxis|VehicleRightLeft`
  (params (AxisValue :type "Float (single-precision)"))
  ;[1 1 1] Vehicle Movement Controls
  (if (`self.AutoGearBox`)
    (`self.GetThrottleInputForAutoHandling` (stale `InputAxis|VehicleForwardBackward` AxisValue) AxisValue)
    (goto _label)
    (else
      (set `self.WheelForwardCoefficient` (`KismetMathLibrary.FClamp` AxisValue))
      (bind _output_get (set `self.BrakeRatioLeft` (* (`KismetMathLibrary.SelectInt` 0 -1 (< AxisValue 0.0)) AxisValue)))
      (set `self.BrakeRatioRight` _output_get)
      (goto _label))))

(event `self.SetRemoveAutoGearBoxTimer`
  (params (bSetTimer :type Boolean))
  ;[1 1 1] Set Remove Auto Gear Box Timer
  (if bSetTimer
    (bind _returnvalue (`KismetSystemLibrary.K2_SetTimer` null "UpdateAutoGearBox" 0.5 true))
    (set `self.AutoGearBoxTimerHandle` _returnvalue)
    (else
      (`KismetSystemLibrary.K2_ClearAndInvalidateTimerHandle` (`self.AutoGearBoxTimerHandle`)))))

(fn `UserConstructionScript`)